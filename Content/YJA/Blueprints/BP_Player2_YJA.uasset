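; Player 2 Blueprint with debug-key test actions for dealing damage and planting seeds.
; L fires a debug-drawn line trace forward from the camera and applies damage to the hit actor.
; Y spawns a BP_Seed at the BP_Pot returned by GetActorOfClass when the player is close to it horizontally.
; Tag-based pickup to the hand socket and trace-based drop logic are present but disconnected, so they never run.
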(event Input|KeyboardEvents|DebugKeyL
  (params (Key :type Key%20Structure :default "None") (ActionValue :type Input%20Action%20Value%20Structure))
  (bind _cameracomponent (Variables|Default|GetCameraComponent))
  (bind _returnvalue (Transformation|GetWorldLocation _cameracomponent))
  (:Pressed
    (bind _outhit (Collision|LineTraceByChannel _returnvalue (+ _returnvalue (* (Math|Vector|GetForwardVector (Transformation|GetWorldRotation _cameracomponent)) (Math|Conversions|ToVector(Float) 1.5e+03))) "TraceTypeQuery2" false 0 "ForDuration" true "(R=1.000000,G=0.000000,B=0.000000,A=1.000000)" "(R=0.000000,G=1.000000,B=0.000000,A=1.000000)" 2.0))
    (Game|Damage|ApplyDamage (.HitActor (Collision|BreakHitResult _outhit)) 1.0 0 self)))

(event Input|KeyboardEvents|DebugKeyY
  (params (Key :type Key%20Structure :default "None") (ActionValue :type Input%20Action%20Value%20Structure))
  (:Pressed
    (bind _returnvalue (Actor|GetActorOfClass "/Game/YJA/Blueprints/BP_Pot.BP_Pot_C"))
    (if (<= (Math|Vector|Distance2D(Vector) (Transformation|GetActorLocation) (Transformation|GetActorLocation _returnvalue)) 8e+01)
      (Game|SpawnActorfromClass "/Game/YJA/Blueprints/BP_Seed.BP_Seed_C" (Math|Transform|MakeTransform (Transformation|GetActorLocation _returnvalue) "0, 0, 0" "1.000000,1.000000,1.000000") "AlwaysSpawn" 0 0))))

(event Input|KeyboardEvents|DebugKeyU
  (params (Key :type Key%20Structure :default "None") (ActionValue :type Input%20Action%20Value%20Structure)))

(fn ConstructionScript)