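; BP_Boat_2 is a boat actor that carries a foundation and tracks whether the player is inside its overlap area.
; On BeginPlay it spawns a BP_Foundation and attaches it to itself, snapping location and rotation while keeping world scale.
; Actor overlap events cast to BP_Player_OSH to toggle the PlayerIn flag, with debug prints; nothing in this graph reads that flag.
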(event EventBeginPlay
  (bind _returnvalue (Game|SpawnActorfromClass "/Game/OSH/Blueprints/Building/BP_Foundation.BP_Foundation_C" (Math|Transform|MakeTransform "0, 0, 0" "0, 0, 0" "1.000000,1.000000,1.000000") "Undefined" 0 0))
  (Transformation|AttachActorToActor _returnvalue self "None" "SnapToTarget" "SnapToTarget" "KeepWorld" true))

(event Collision|EventActorBeginOverlap
  (params (OtherActor :type Actor%20Object%20Reference))
  (Development|PrintString "Begin")
  (Utilities|Casting|CastToBP_Player_OSH OtherActor)
  (Variables|Default|SetPlayerIn true)
  (Development|PrintString "In"))

(event EventTick
  (params (DeltaSeconds :type Float%20%28single-precision%29)))

(event Collision|EventActorEndOverlap
  (params (OtherActor :type Actor%20Object%20Reference))
  (Development|PrintString "End")
  (Utilities|Casting|CastToBP_Player_OSH OtherActor)
  (Variables|Default|SetPlayerIn false)
  (Development|PrintString "Out"))

(fn ConstructionScript)