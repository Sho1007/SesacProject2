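; Shark character Blueprint, apparently a work-in-progress prototype of an enemy that roams, chases the player and reacts to the boat.
; BeginPlay finds BP_BoatTest and, if the player is aboard, sets the shark's location to a normalized direction vector.
; Custom events cover AI random roaming, chasing by snapping to the player, and montage attacks; boat-circling is empty.
; Tick is empty, and the cooldown, distance and state-selection logic is disconnected.
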(event Custom|Roaming
  (Development|PrintString "Roaming")
  (Variables|Default|SetbIsMoving true)
  (Variables|/Script/Engine.CharacterMovementComponent|SetMaxWalkSpeed (Variables|Character|GetCharacterMovement) 2e+02)
  (AI|AIMoveTo self (.RandomLocation (AI|Navigation|GetRandomReachablePointinRadius (Transformation|GetActorLocation) 9e+05 0 0)) 0 5.0 false
    (:OnSuccess
      (Variables|Default|SetbIsMoving false))))

(event Custom|ChasingPlayer
  (Development|PrintString "Chasing")
  (Variables|/Script/Engine.CharacterMovementComponent|SetMaxWalkSpeed (Variables|Character|GetCharacterMovement) 4.5e+02)
  (Transformation|SetActorLocation (Transformation|GetActorLocation (Game|GetPlayerCharacter 0)) false false))

(event Custom|RoamingAroundBoat)

(event Custom|AttackPlayer
  (Animation|Montage|PlayMontage (Variables|Character|GetMesh) 0))

(event Collision|EventActorBeginOverlap
  (params (OtherActor :type Actor%20Object%20Reference))
  (Development|PrintString "overlap")
  (Variables|Default|SetCurrentCoolTime 0.0)
  (Variables|Default|SetbAttackable false))

(event EventBeginPlay
  (bind _returnvalue (Actor|GetActorOfClass "/Game/YJA/Blueprints/BP_BoatTest.BP_BoatTest_C"))
  (Variables|Default|SetBoat _returnvalue)
  (bind _output_get (Variables|Default|SetDirection (Math|Vector|Normalize (- (Transformation|GetActorLocation _returnvalue) (Transformation|GetActorLocation)))))
  (if (Variables|/Game/YJA/Blueprints/BP_BoatTest.BP_BoatTest_C|GetPlayerIn (Variables|Default|GetBoat))
    (Transformation|SetActorLocation (Math|Vector|Normalize (* (Utilities|Time|GetWorldDeltaSeconds) (* _output_get (Variables|Default|GetSpeed)))) false false)))

(event EventTick
  (params (DeltaSeconds :type Float%20%28single-precision%29)))

(fn ConstructionScript)