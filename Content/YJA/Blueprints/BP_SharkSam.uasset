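; Shark enemy that circles BP_Boat_2 and charges it, switching to chase the player character whenever they leave the boat.
; A Tick-driven enum state machine cycles from timed Roaming to AttackBoat, then to Back after lingering within attack range, retreating until far enough to roam again.
; Damage also sets Back; no damage is dealt here.
; Flying mode is set, but motion uses look-at rotations and unswept world offsets, circling perpendicular to the boat.
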(event EventBeginPlay
  ;[0.152 0.6067 1] BeginPlay
  (Development|PrintString "BeginPlay")
  (bind _returnvalue (Actor|GetActorOfClass "/Script/MarineCraft.Boat"))
  (bind _asbp_boat_2 (Utilities|Casting|CastToBP_Boat_2 _returnvalue))
  (Variables|Default|SetBoat _asbp_boat_2)
  (Pawn|Components|CharacterMovement|SetMovementMode (Variables|Character|GetCharacterMovement) "MOVE_Flying" 0))

(event EventTick
  (params (DeltaSeconds :type Float%20%28single-precision%29))
  (bind _returnvalue (Transformation|GetActorLocation))
  (bind _returnvalue_2 (Transformation|GetActorLocation))
  (CallFunction|CalculateBoatDistance)
  (if (Variables|/Game/YJA/Blueprints/BP_Boat_2.BP_Boat_2_C|GetPlayerIn (Variables|Default|GetBoat))
    _
    (else
      (Variables|Default|SetState "NewEnumerator9")))
  (switch Utilities|FlowControl|Switch|SwitchonE_Shark (Variables|Default|GetState)
    (:NewEnumerator7
      (CallFunction|Back))
    (:NewEnumerator8
      (CallFunction|RoamingBoat)
      (bind _output_get (Variables|Default|SetCurrentRoamTime (+ (Variables|Default|GetCurrentRoamTime) DeltaSeconds)))
      (if (>= _output_get (Variables|Default|GetMaxRoamTime))
        (Variables|Default|SetCurrentRoamTime 0.0)
        (Variables|Default|SetState "NewEnumerator10")))
    (:NewEnumerator9
      (if (Variables|/Game/YJA/Blueprints/BP_Boat_2.BP_Boat_2_C|GetPlayerIn (Variables|Default|GetBoat))
        (Variables|Default|SetState "NewEnumerator10")
        (elif (not (Variables|Default|GetbIsMoving))
          (Variables|Default|SetbIsMoving true)
          (Variables|/Script/Engine.CharacterMovementComponent|SetMaxWalkSpeed (Variables|Character|GetCharacterMovement) 4.5e+02)
          (Transformation|SetActorRotation (Math|Rotator|FindLookatRotation _returnvalue_2 (+ _returnvalue_2 (- (Transformation|GetActorLocation (Game|GetPlayerCharacter 0)) (Transformation|GetActorLocation)))))
          (Transformation|AddActorWorldOffset (* (Transformation|GetActorForwardVector) (Utilities|Time|GetWorldDeltaSeconds) (Variables|/Script/Engine.CharacterMovementComponent|GetMaxWalkSpeed (Variables|Character|GetCharacterMovement))))
          (Variables|Default|SetbIsMoving false))))
    (:NewEnumerator10
      (Variables|/Script/Engine.CharacterMovementComponent|SetMaxWalkSpeed (Variables|Character|GetCharacterMovement) 4.5e+02)
      (if (Variables|/Game/YJA/Blueprints/BP_Boat_2.BP_Boat_2_C|GetPlayerIn (Variables|Default|GetBoat))
        (Transformation|SetActorRotation (Math|Rotator|FindLookatRotation _returnvalue (+ _returnvalue (- (Transformation|GetActorLocation (Variables|Default|GetBoat)) (Transformation|GetActorLocation)))))
        (if (< (Variables|Default|GetBoatDistance) (Variables|Default|GetAttackDistance))
          (bind _output_get_2 (Variables|Default|SetCurrentAttackTime (+ (Variables|Default|GetCurrentAttackTime) (Utilities|Time|GetWorldDeltaSeconds))))
          (if (>= _output_get_2 (Variables|Default|GetMaxAttackTime))
            (Variables|Default|SetCurrentAttackTime 0.0)
            (Variables|Default|SetState "NewEnumerator7"))
          (else
            (Transformation|AddActorWorldOffset (* (Transformation|GetActorForwardVector) (Utilities|Time|GetWorldDeltaSeconds) (Variables|/Script/Engine.CharacterMovementComponent|GetMaxWalkSpeed (Variables|Character|GetCharacterMovement))))))
        (else
          (Variables|Default|SetState "NewEnumerator9"))))))

(event Game|Damage|EventAnyDamage
  (params (Damage :type Float%20%28single-precision%29) (DamageType :type Damage%20Type%20Object%20Reference) (InstigatedBy :type Controller%20Object%20Reference) (DamageCauser :type Actor%20Object%20Reference))
  ;[1 0.2816 0.6353] Damage
  (Variables|Default|SetState "NewEnumerator7"))

(fn ConstructionScript)

(fn BoatinTime)

(fn AngleTimeFunc
  (bind _output_get (Variables|Default|SetCurrentTime (+ (Utilities|Time|GetWorldDeltaSeconds) (Variables|Default|GetCurrentTime))))
  (return (> _output_get (Variables|Default|GetChangeAngleTime))))

(fn RoamingBoat
  (bind _returnvalue (Transformation|GetActorLocation))
  (Variables|/Script/Engine.CharacterMovementComponent|SetMaxWalkSpeed (Variables|Character|GetCharacterMovement) 4.5e+02)
  (Transformation|SetActorRotation (Math|Rotator|FindLookatRotation _returnvalue (+ _returnvalue (Math|Vector|RotateVector (- (Transformation|GetActorLocation (Variables|Default|GetBoat)) (Transformation|GetActorLocation)) "0.000000,90.000000,0.000000"))))
  (Transformation|AddActorWorldOffset (* (Transformation|GetActorForwardVector) (Utilities|Time|GetWorldDeltaSeconds) (Variables|Default|GetSpeed))))

(fn RotatetoBack
  (bind _returnvalue (Transformation|GetActorLocation))
  (Variables|/Script/Engine.CharacterMovementComponent|SetMaxWalkSpeed (Variables|Character|GetCharacterMovement) 1.5e+02)
  (Transformation|SetActorRotation (Math|Rotator|FindLookatRotation _returnvalue (+ _returnvalue (- (Transformation|GetActorLocation) (Transformation|GetActorLocation (Variables|Default|GetBoat))))))
  (return))

(fn CalculateBoatDistance
  (Variables|Default|SetBoatDistance (Math|Vector|VectorLength (- (Transformation|GetActorLocation) (Transformation|GetActorLocation (Variables|Default|GetBoat)))))
  (return))

(fn Back
  (CallFunction|RotatetoBack)
  (Transformation|AddActorWorldOffset (* (Transformation|GetActorForwardVector) (Utilities|Time|GetWorldDeltaSeconds) (Variables|/Script/Engine.CharacterMovementComponent|GetMaxWalkSpeed (Variables|Character|GetCharacterMovement))))
  (if (>= (Variables|Default|GetBoatDistance) 1.5e+03)
    (Variables|Default|SetState "NewEnumerator8")))