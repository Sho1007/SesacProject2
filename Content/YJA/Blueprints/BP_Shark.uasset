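; BP_Shark is an AI shark character that roams randomly and chases the player when nearby.
; Tick checks the BP_Boat found at BeginPlay: a boarded player routes to an empty RoamingAroundBoat stub, otherwise 2D distance selects a faster AIMoveTo chase or slower random roaming.
; Any actor overlap starts a cooldown, during which the shark only roams until it can attack again.
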(event Custom|Roaming
  (Development|PrintString "Roaming")
  (Variables|Default|SetbIsMoving true)
  (Variables|/Script/Engine.CharacterMovementComponent|SetMaxWalkSpeed (Variables|Character|GetCharacterMovement) 2e+02)
  (AI|AIMoveTo self (.RandomLocation (AI|Navigation|GetRandomReachablePointinRadius (Transformation|GetActorLocation) 9e+05 0 0)) 0 5.0 false
    (:OnSuccess
      (Variables|Default|SetbIsMoving false))))

(event Custom|ChasingPlayer
  (Development|PrintString "Chasing")
  (Variables|/Script/Engine.CharacterMovementComponent|SetMaxWalkSpeed (Variables|Character|GetCharacterMovement) 4.5e+02)
  (AI|AIMoveTo self (Transformation|GetActorLocation) (Game|GetPlayerCharacter 0) 5.0 false))

(event Custom|RoamingAroundBoat)

(event Collision|EventActorBeginOverlap
  (params (OtherActor :type Actor%20Object%20Reference))
  (Development|PrintString "overlap")
  (Variables|Default|SetCurrentCoolTime 0.0)
  (Variables|Default|SetbAttackable false))

(event EventBeginPlay
  (bind _returnvalue (Actor|GetActorOfClass "/Game/YJA/Blueprints/BP_Boat.BP_Boat_C"))
  (Variables|Default|SetTargetBoat _returnvalue))

(event EventTick
  (params (DeltaSeconds :type Float%20%28single-precision%29))
  (if (Variables|Default|GetbAttackable)
    (if (Variables|/Game/YJA/Blueprints/BP_Boat.BP_Boat_C|GetPlayerIn (Variables|Default|GetTargetBoat)) :!label _label
      (CallFunction|RoamingAroundBoat)
      (elif (< (Math|Vector|Distance2D(Vector) (Transformation|GetActorLocation) (Transformation|GetActorLocation (Game|GetPlayerCharacter 0))) 1.5e+03)
        (Variables|Default|SetbIsMoving false)
        (if (Variables|Default|GetbAttackable)
          (CallFunction|ChasingPlayer))
        (elif (not (Variables|Default|GetbIsMoving))
          (CallFunction|Roaming))))
    (else
      (bind _output_get (Variables|Default|SetCurrentCoolTime (+ DeltaSeconds (Variables|Default|GetCurrentCoolTime))))
      (if (>= _output_get (Variables|Default|GetCoolTime))
        (Variables|Default|SetbAttackable true)
        (goto _label)
        (else
          (CallFunction|Roaming))))))

(fn ConstructionScript)