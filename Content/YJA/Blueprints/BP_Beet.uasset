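; BP_Beet is a beet crop actor that grows from zero scale toward full size over a set growth time.
; BeginPlay shrinks the actor to zero, then Tick accumulates delta time and scales the root by the fraction of maximum growth reached.
; Once growth completes, it disables its own Tick and switches the Box to query-only collision.
; The overlap event is empty.
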(event EventBeginPlay
  (Transformation|SetActorScale3D "0, 0, 0"))

(event Collision|EventActorBeginOverlap
  (params (OtherActor :type Actor%20Object%20Reference)))

(event EventTick
  (params (DeltaSeconds :type Float%20%28single-precision%29))
  (bind _output_get (Variables|Default|SetCurrentBeetGrowth (+ DeltaSeconds (Variables|Default|GetCurrentBeetGrowth))))
  (if (>= _output_get (Variables|Default|GetCurrentBeetMaxGrowth))
    (Actor|Tick|SetActorTickEnabled false)
    (Collision|SetCollisionEnabled (Variables|Default|GetBox) "QueryOnly")
    (else
      (Transformation|SetWorldScale3D (Variables|Default|GetDefaultSceneRoot) (Math|Conversions|ToVector(Float) (/ (Variables|Default|GetCurrentBeetGrowth) (Variables|Default|GetCurrentBeetMaxGrowth)))))))

(fn ConstructionScript)