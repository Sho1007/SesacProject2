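; Player character Blueprint that switches between walking and swimming as it moves through water, and handles jump input.
; Water enter/exit events set a flag and record the entry height as the surface level.
; While in water, Tick compares depth below that level to capsule half-height plus a margin, toggling movement mode and physics-volume water through two mutually resetting DoOnce gates.
; Pitch-rotation and still-in-water logic is left unconnected.
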(event EventBeginPlay)

(event Collision|EventActorBeginOverlap
  (params (OtherActor :type Actor%20Object%20Reference)))

(event EventTick
  (params (DeltaSeconds :type Float%20%28single-precision%29))
  (CallFunction|Swimming))

(event EventEnterWater
  (Variables|Default|SetisInWater true)
  (Variables|Default|SetWaterZ (.z (Transformation|GetActorLocation))))

(event EventExitWater
  (Variables|Default|SetisInWater false))

(event Input|ActionEvents|InputActionJump
  (params (Key :type Key%20Structure :default "None"))
  (:Pressed
    (Character|Jump)))

(fn ConstructionScript)

(fn Swimming
  (bind _charactermovement (Variables|Character|GetCharacterMovement))
  (bind _charactermovement_2 (Variables|Character|GetCharacterMovement))
  (if (Variables|Default|GetisInWater)
    (if (CallFunction|SeaLevelHigh)
      ;[1 1 1] 바다에서 : Swim
      (Utilities|FlowControl|DoOnce false :!label _label
        (:Completed
          (Variables|/Script/Engine.PhysicsVolume|SetbWaterVolume (Class|MovementComponent|GetPhysicsVolume _charactermovement_2) true)
          (Pawn|Components|CharacterMovement|SetMovementMode _charactermovement_2 "MOVE_Swimming" 0)
          (goto _label_2 Reset)))
      (else
        ;[1 1 1] 육지에서 : Walk
        (if (CallFunction|SeaLevelLow)
          (Utilities|FlowControl|DoOnce false :!label _label_2
            (:Completed
              (Variables|/Script/Engine.PhysicsVolume|SetbWaterVolume (Class|MovementComponent|GetPhysicsVolume _charactermovement) false)
              (Pawn|Components|CharacterMovement|SetMovementMode _charactermovement "MOVE_Walking" 0)
              (goto _label Reset))))))))

(fn SeaLevelLow
  (return (< (- (Variables|Default|GetWaterZ) (.z (Transformation|GetActorLocation))) (+ (Variables|/Script/Engine.CapsuleComponent|GetCapsuleHalfHeight (Variables|Default|GetCapsuleComponent)) 3e+01))))

(fn SeaLevelHigh
  (return (> (- (Variables|Default|GetWaterZ) (.z (Transformation|GetActorLocation))) (+ (Variables|/Script/Engine.CapsuleComponent|GetCapsuleHalfHeight (Variables|Default|GetCapsuleComponent)) 3e+01))))

(fn StillinWater
  (Variables|Default|SetisStillInWater (or (CallFunction|SeaLevelHigh) (CallFunction|SeaLevelLow)))
  (return))