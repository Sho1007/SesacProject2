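; BP_Foundation is the foundation piece of a building system, defining box components for Floor and Wall parts.
; On BeginPlay it adds two BuildBox structs to BuildBoxArray, each pairing a part name with its four matching boxes.
; The file only registers this data; it contains no placement logic, and its construction script is empty.
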(event EventBeginPlay
  (Utilities|Array|Add (Variables|Default|GetBuildBoxArray) (Utilities|Struct|MakeBuildBox "Floor" (Utilities|Array|MakeArray (Variables|Default|GetFloorBox1) (Variables|Default|GetFloorBox2) (Variables|Default|GetFloorBox3) (Variables|Default|GetFloorBox4))))
  (Utilities|Array|Add (Variables|Default|GetBuildBoxArray) (Utilities|Struct|MakeBuildBox "Wall" (Utilities|Array|MakeArray (Variables|Default|GetWallBox1) (Variables|Default|GetWallBox2) (Variables|Default|GetWallBox3) (Variables|Default|GetWallBox4)))))

(fn ConstructionScript)