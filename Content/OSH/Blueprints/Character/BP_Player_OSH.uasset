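; BP_Player_OSH is a player Blueprint that adds debug tooling for on-screen messages and inventory testing.
; On BeginPlay it creates a WBP_DebugUI widget and adds it to the viewport, and MyPrintLog_1 writes its message into that widget's text block.
; Debug keys each spawn an item actor (flotsam plank or plastic, rope, raw potato) and add it to the InventoryComponent.
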(event Custom|MyPrintLog_1
  (params (message :type String))
  (Variables|/Script/UMG.TextBlock|SetText (Variables|/Game/OSH/Level/WBP_DebugUI.WBP_DebugUI_C|GetTextBlock_1 (Variables|Default|GetNewVar)) (Utilities|Text|ToText(String) message)))

(event EventBeginPlay
  (bind _returnvalue (UserInterface|CreateWidget "/Game/OSH/Level/WBP_DebugUI.WBP_DebugUI_C"))
  (bind _output_get (Variables|Default|SetNewVar _returnvalue))
  (UserInterface|Viewport|AddtoViewport _output_get 0))

(event Collision|EventActorBeginOverlap
  (params (OtherActor :type Actor%20Object%20Reference)))

(event EventTick
  (params (DeltaSeconds :type Float%20%28single-precision%29)))

(event Input|KeyboardEvents|DebugKeyL
  (params (Key :type Key%20Structure :default "None") (ActionValue :type Input%20Action%20Value%20Structure))
  (:Pressed
    (bind _returnvalue (Game|SpawnActorfromClass "/Game/OSH/Blueprints/Inventory/Food/BP_RawPotato.BP_RawPotato_C" (Math|Transform|MakeTransform "0, 0, 0" "0, 0, 0" "1.000000,1.000000,1.000000") "Undefined" 0 0))
    (Class|PlayerInventoryComponent|AddItem (Variables|Default|GetInventoryComponent) _returnvalue)))

(event Input|KeyboardEvents|DebugKeyH
  (params (Key :type Key%20Structure :default "None") (ActionValue :type Input%20Action%20Value%20Structure))
  (:Pressed
    (bind _returnvalue (Game|SpawnActorfromClass "/Game/OSH/Blueprints/Inventory/Floatsam/BP_Floatsam_Plank.BP_Floatsam_Plank_C" (Math|Transform|MakeTransform "0, 0, 0" "0, 0, 0" "1.000000,1.000000,1.000000") "Undefined" 0 0))
    (Class|PlayerInventoryComponent|AddItem (Variables|Default|GetInventoryComponent) _returnvalue)))

(event Input|KeyboardEvents|DebugKeyJ
  (params (Key :type Key%20Structure :default "None") (ActionValue :type Input%20Action%20Value%20Structure))
  (:Pressed
    (bind _returnvalue (Game|SpawnActorfromClass "/Game/OSH/Blueprints/Inventory/Floatsam/BP_Floatsam_Plastic.BP_Floatsam_Plastic_C" (Math|Transform|MakeTransform "0, 0, 0" "0, 0, 0" "1.000000,1.000000,1.000000") "Undefined" 0 0))
    (Class|PlayerInventoryComponent|AddItem (Variables|Default|GetInventoryComponent) _returnvalue)))

(event Input|KeyboardEvents|DebugKeyK
  (params (Key :type Key%20Structure :default "None") (ActionValue :type Input%20Action%20Value%20Structure))
  (:Pressed
    (bind _returnvalue (Game|SpawnActorfromClass "/Game/OSH/Blueprints/Inventory/BP_Rope.BP_Rope_C" (Math|Transform|MakeTransform "0, 0, 0" "0, 0, 0" "1.000000,1.000000,1.000000") "Undefined" 0 0))
    (Class|PlayerInventoryComponent|AddItem (Variables|Default|GetInventoryComponent) _returnvalue)))

(fn ConstructionScript)