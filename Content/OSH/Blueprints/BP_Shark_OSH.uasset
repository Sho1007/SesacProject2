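; BP_Shark_OSH is a shark actor that circles the boat, the first BP_Foundation found at BeginPlay.
; Each Tick it faces a rotated offset of its vector to the boat and moves forward by Speed without sweep, producing orbit-like motion.
; Helper functions measure boat distance, steer straight at the boat or turn sideways, but the event graph calls none of them.
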(event EventBeginPlay
  ;[1 1 1] BeginPlay
  (bind _returnvalue (Actor|GetActorOfClass "/Game/OSH/Blueprints/Building/BP_Foundation.BP_Foundation_C"))
  (Variables|Default|SetBoat _returnvalue))

(event EventTick
  (params (DeltaSeconds :type Float%20%28single-precision%29))
  (bind _returnvalue (Transformation|GetActorLocation))
  (Transformation|SetActorRotation (Math|Rotator|FindLookatRotation _returnvalue (+ _returnvalue (Math|Vector|RotateVector (- (Transformation|GetActorLocation (Variables|Default|GetBoat)) (Transformation|GetActorLocation)) "0.000000,90.000000,0.000000"))))
  (Transformation|AddActorWorldOffset (* (Transformation|GetActorForwardVector) DeltaSeconds (Variables|Default|GetSpeed))))

(fn ConstructionScript)

(fn GetBoatDistance
  (Variables|Default|SetBoatDistance (Math|Vector|VectorLength (- (Transformation|GetActorLocation (Variables|Default|GetBoat)) (Transformation|GetActorLocation))))
  (return))

(fn MovetoBoat
  (params (B :type Float%20%28single-precision%29))
  (Transformation|SetActorRotation (Math|Rotator|FindLookatRotation (Transformation|GetActorLocation) (Transformation|GetActorLocation (Variables|Default|GetBoat))))
  (Transformation|AddActorWorldOffset (* (Transformation|GetActorForwardVector) B (Variables|Default|GetSpeed))))

(fn Turn
  (bind _returnvalue (Transformation|GetActorLocation))
  (Transformation|SetActorRotation (Math|Rotator|FindLookatRotation _returnvalue (Math|Vector|RotateVectorAroundAxis (+ (- (Transformation|GetActorLocation (Variables|Default|GetBoat)) _returnvalue) _returnvalue) 9e+01 "0.000000,0.000000,1.000000"))))